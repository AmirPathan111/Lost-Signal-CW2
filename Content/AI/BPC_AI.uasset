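; AI enemy pawn that feeds player detection and attack-range state to its Blackboard.
; Each Tick recomputes the vector to the player and compares its length with AttackRange and PawnSensing's SightRadius to set "IsInAttackRange?" and "CanSeePlayer?".
; The sight flag updates only if the last seen pawn casts to BP_FirstPersonCharacter, and then by distance alone.
; OnSeePawn also schedules that check on a short timer, alongside the per-Tick call.
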(event `GetDistance`
  (set `self.distance` (- (`self.K2_GetActorLocation` (`GameplayStatics.GetPlayerCharacter` 0)) (`self.K2_GetActorLocation`))))

(event `self.ReceiveTick`
  (params (DeltaSeconds :type "Float (single-precision)"))
  (`self.AttackPlayer`)
  (`self.LOS`)
  (`self.GetDistance`))

(event `AttackPlayer`
  (bind _returnvalue (`AIBlueprintHelperLibrary.GetBlackboard` (`AIBlueprintHelperLibrary.GetAIController` self)))
  (if (<= (`KismetMathLibrary.VSize` (`self.distance`)) (`self.AttackRange`))
    (`BlackboardComponent.SetValueAsBool` _returnvalue "IsInAttackRange?" true)
    (else
      (`BlackboardComponent.SetValueAsBool` _returnvalue "IsInAttackRange?" false))))

(event `self.PawnSensing.OnSeePawn`
  (params (Pawn :type "Pawn Object Reference"))
  (`KismetSystemLibrary.K2_SetTimerDelegate` (delegate `LOS`) 1.5))

(event `LOS`
  (bind _returnvalue (`AIBlueprintHelperLibrary.GetBlackboard` (`AIBlueprintHelperLibrary.GetAIController` self)))
  (cast `/Game/FirstPerson/Blueprints/BP_FirstPersonCharacter` (stale `self.PawnSensing.OnSeePawn` Pawn))
  (if (<= (`KismetMathLibrary.VSize` (`self.distance`)) (`PawnSensingComponent.SightRadius` (`self.PawnSensing`)))
    (`BlackboardComponent.SetValueAsBool` _returnvalue "CanSeePlayer?" true)
    (else
      (`BlackboardComponent.SetValueAsBool` _returnvalue "CanSeePlayer?" false))))

(fn `UserConstructionScript`)