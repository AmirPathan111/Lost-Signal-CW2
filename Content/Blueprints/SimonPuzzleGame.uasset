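; Simon Says puzzle actor that hosts a SimonSaysInterface screen in a widget component and shows the player a colour sequence.
; On BeginPlay it binds the four colour buttons, switches input to UI-only with a visible cursor, then displays the current stage's colours from ColourOrder.
; Button clicks only print their colour, with no sequence checking, and the display starts on BeginPlay rather than on interaction.
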(event `self.ReceiveBeginPlay`
  (bind _returnvalue (`GameplayStatics.GetPlayerController` 0))
  (bind _returnvalue_2 (`WidgetComponent.GetWidget` (`self.Widget`)))
  ;[1 1 1] Casting to the puzzle screen to get the on clicked events
  (bind _assimon_says_interface (cast `/Game/UserInterface/SimonSaysInterface` _returnvalue_2))
  (add `Button.OnClicked` (`/Game/UserInterface/SimonSaysInterface.YellowButton` _assimon_says_interface) (delegate `YellowClicked`))
  (bind _assimon_says_interface_2 (cast `/Game/UserInterface/SimonSaysInterface` _returnvalue_2))
  (add `Button.OnClicked` (`/Game/UserInterface/SimonSaysInterface.GreenButton` _assimon_says_interface_2) (delegate `GreenClicked`))
  (bind _assimon_says_interface_3 (cast `/Game/UserInterface/SimonSaysInterface` _returnvalue_2))
  (add `Button.OnClicked` (`/Game/UserInterface/SimonSaysInterface.RedButton` _assimon_says_interface_3) (delegate `RedClicked`))
  (bind _assimon_says_interface_4 (cast `/Game/UserInterface/SimonSaysInterface` _returnvalue_2))
  (add `Button.OnClicked` (`/Game/UserInterface/SimonSaysInterface.BlueButton` _assimon_says_interface_4) (delegate `BlueClicked`))
  (`KismetSystemLibrary.PrintString` "All Casting done")
  ;[1 1 1] Make interface interactable
  (`WidgetBlueprintLibrary.SetInputMode_UIOnlyEx` _returnvalue (`WidgetComponent.GetWidget` (`self.Widget`)) "DoNotLock" true)
  (set `PlayerController.bShowMouseCursor` true _returnvalue)
  ;[1 1 1] Show colours on screen
  (message `/Game/Blueprints/Interfaces/ColoursArrayInterface.Show Colours In Display` (`WidgetComponent.GetWidget` (`self.Widget`)) (`.colours` (break `ColourOrder` (`|GetArrayItem` (`self.ColourOrder`) (`self.currentStage`))))) ; Should be changed to on interact
)

(event `YellowClicked`
  ;[1 1 1] OnClicked Events
  (`KismetSystemLibrary.PrintString` "Yellow"))

(event `GreenClicked`
  ;[1 1 1] OnClicked Events
  (`KismetSystemLibrary.PrintString` "Green"))

(event `RedClicked`
  ;[1 1 1] OnClicked Events
  (`KismetSystemLibrary.PrintString` "Red"))

(event `BlueClicked`
  ;[1 1 1] OnClicked Events
  (`KismetSystemLibrary.PrintString` "Blue"))

(fn `UserConstructionScript`)