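; Interactable spot-the-difference puzzle terminal that opens a sci-fi door when its puzzle is completed.
; On BeginPlay it creates the puzzle widget from its image and answer variables, passes itself to it and binds to PuzzleCompleted.
; Overlap toggles the interaction prompt, and Interact shows the widget with UI-only input and a mouse cursor.
; Completion removes the widget, restores game input and snaps the door to a fixed rotation.
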(event `self.ReceiveActorBeginOverlap`
  (params (OtherActor :type "Actor Object Reference"))
  (`SceneComponent.SetVisibility` (`self.Interaction`) true false))

(event `self.ReceiveActorEndOverlap`
  (params (OtherActor :type "Actor Object Reference"))
  (`SceneComponent.SetVisibility` (`self.Interaction`) false false))

(event `self.ReceiveBeginPlay`
  (bind _returnvalue (`|CreateWidget` "/Game/Puzzles/SpotTheDifferencePuzzle.SpotTheDifferencePuzzle_C" (`GameplayStatics.GetPlayerController` 0) (`self.Image Left`) (`self.Image Left 1`) (`self.Image Left 2`) (`self.Image Middle`) (`self.Image Middle 1`) (`self.Image Middle 2`) (`self.Image Right`) (`self.Image Right 1`) (`self.Image Right 2`) (`self.The Answer`)))
  (bind _output_get (set `self.Uiwidget` _returnvalue))
  (`/Game/Puzzles/SpotTheDifferencePuzzle.SaveTerminalObject` _output_get self)
  (add `self.PuzzleCompleted` (delegate `PuzzleCompleted_Event`)))

(event `/Game/FirstPerson/Blueprints/Interface/Interact_Interface.Interact`
  (`UserWidget.AddToViewport` (`self.Uiwidget`) 0)
  (`WidgetBlueprintLibrary.SetInputMode_UIOnlyEx` (`GameplayStatics.GetPlayerController` 0) null)
  (set `PlayerController.bShowMouseCursor` true (`GameplayStatics.GetPlayerController` 0)))

(event `PuzzleCompleted_Event`
  (bind _returnvalue (`GameplayStatics.GetPlayerController` 0))
  (`KismetSystemLibrary.PrintString` "Hello")
  (set `PlayerController.bShowMouseCursor` false _returnvalue)
  (`WidgetBlueprintLibrary.SetInputMode_GameOnly` _returnvalue)
  (`Widget.RemoveFromParent` (`self.Uiwidget`))
  (`SceneComponent.K2_SetWorldRotation` (`self.SM_Scifi_Door_02`) (struct :`Yaw` -90.0) false false))

(fn `UserConstructionScript`)